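; BP_Player is the player in CubeRunner, pushed constantly forward by physics impulses and steered sideways by the MoveRight axis.
; It creates the HUD on BeginPlay and caches BP_GameModeBase to report results.
; Hitting a BP_Obstacle or dropping below zero height calls EndGame, while overlapping BP_EndPoint calls LevelComplete.
; The IsLife flag gates movement and prevents repeated game-over calls.
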(event `self.ReceiveBeginPlay`
  (bind _returnvalue (`|CreateWidget` "/Game/CubeRunner_V2/Core/HUD/WBP_HUD.WBP_HUD_C" (`GameplayStatics.GetPlayerController` 0)))
  (bind _output_get (set `self.WBP_HUD` _returnvalue))
  (`UserWidget.AddToViewport` _output_get 0)
  (bind _asbp_game_mode_base (cast `/Game/CubeRunner_V2/Core/Blueprints/BP_GameModeBase` (`GameplayStatics.GetGameMode`)))
  (set `self.GameModeRef` _asbp_game_mode_base))

(event `InputAxis|MoveRight`
  (params (AxisValue :type "Float (single-precision)"))
  (set `self.MovOrient` AxisValue)
  (if (`self.isLife`)
    (`PrimitiveComponent.AddImpulse` (`self.Player`) (`KismetMathLibrary.MakeVector` (* (`self.SideForce`) (`self.MovOrient`))) "None" true)))

(event `self.ReceiveTick`
  (params (DeltaSeconds :type "Float (single-precision)"))
  (bind (_returnvalue_x _returnvalue_y _returnvalue_z) (`KismetMathLibrary.BreakVector` (`self.K2_GetActorLocation`)))
  (if (`self.isLife`)
    (`PrimitiveComponent.AddImpulse` (`self.Player`) (`KismetMathLibrary.MakeVector` 0.0 (`self.ForwardForce`)) "None" true)
    (if (< _returnvalue_z 0.0)
      (`self.GameEnded`))))

(event `self.Player.OnComponentHit`
  (params (HitComponent :type "PrimitiveComponent Object Reference") (OtherActor :type "Actor Object Reference") (OtherComp :type "PrimitiveComponent Object Reference") (NormalImpulse :type "Vector Structure") (Hit :type "HitResult Structure (by ref)"))
  (cast `/Game/CubeRunner_V2/Core/Blueprints/BP_Obstacle` OtherActor)
  (`self.GameEnded`))

(event `self.Player.OnComponentBeginOverlap`
  (params (OverlappedComponent :type "PrimitiveComponent Object Reference") (OtherActor :type "Actor Object Reference") (OtherComp :type "PrimitiveComponent Object Reference") (OtherBodyIndex :type Integer) (bFromSweep :type Boolean) (SweepResult :type "HitResult Structure (by ref)"))
  (cast `/Game/CubeRunner_V2/Core/Blueprints/BP_EndPoint` OtherActor)
  (set `self.isLife` false)
  (`/Game/CubeRunner_V2/Core/Blueprints/BP_GameModeBase.LevelComplete` (`self.GameModeRef`)))

(fn `GameEnded`
  (if (`self.isLife`)
    (set `self.isLife` false)
    (`/Game/CubeRunner_V2/Core/Blueprints/BP_GameModeBase.EndGame` (`self.GameModeRef`))))

(fn `UserConstructionScript`)